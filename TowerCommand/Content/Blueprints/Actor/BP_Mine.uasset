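; BP_Mine is a mine, which a sub can lay, that homes in on nearby targets and explodes.
; Each tick it applies force toward every BPI_Targetable actor within homing distance except its instigator, scaled by inverse distance.
; Hits or damage trigger an authority-only explosion that fires a radial impulse, applies falloff damage and destroys the mine, guarded against chain-reaction loops.
; Destruction spawns the explosion effect.
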(event EventBeginPlay)

(event EventActorBeginOverlap
  (params (OtherActor :type Actor%20Object%20Reference)))

(event EventTick
  (params (DeltaSeconds :type Float%20%28single-precision%29))
  ;[1 1 1] Per-frame processing.
  (bind _outactors (Actor|GetAllActorswithInterface "/Game/Blueprints/Attributes/BPI_Targetable.BPI_Targetable_C"))
  (for _array_element _outactors ; Find the closest targetable actors\n(that aren't this mine) and add\nforces to push the mine to those\nthat are close enough.
    (if (!= self _array_element) ; Mine can't target itself.
      (if (!= (Game|GetInstigator) _array_element) ; Mine doesn't target sub that laid it (if any).
        (if (< (Transformation|GetDistanceTo _array_element) (Variables|Default|GetHoming%20Distance)) ; If target within homing distance, home in on it!
          (Physics|AddForce (* (Class|KismetMathLibrary|GetDirectionVector (Transformation|GetActorLocation) (Transformation|GetActorLocation _array_element)) (/ (Variables|Default|GetHoming%20Force) (Transformation|GetDistanceTo _array_element))) "None") ; The force applied is proportional to the inverse\nof distance (square distance was too high)\nand boosted by a 'homing force' scale factor.
        )))))

(event EventHit
  (params (MyComp :type Primitive%20Component%20Object%20Reference) (Other :type Actor%20Object%20Reference) (OtherComp :type Primitive%20Component%20Object%20Reference) (bSelfMoved :type Boolean) (HitLocation :type Vector :default "0, 0, 0") (HitNormal :type Vector :default "0, 0, 0") (NormalImpulse :type Vector :default "0, 0, 0") (Hit :type Hit%20Result%20Structure%20%28by%20ref%29))
  ;[1 1 1] Explode if hit by another object or explosion.
  (CallFunction|ExplodeonHit))

(event EventAnyDamage
  (params (Damage :type Float%20%28single-precision%29) (DamageType :type Damage%20Type%20Object%20Reference) (InstigatedBy :type Controller%20Object%20Reference) (DamageCauser :type Actor%20Object%20Reference))
  ;[1 1 1] Explode if hit by another object or explosion.
  (CallFunction|ExplodeonHit))

(event EventDestroyed
  ;[1 1 1] Explode if hit by another object or explosion.
  (Game|SpawnActorfromClass "/Game/Blueprints/Blueprint_Effect_Explosion.Blueprint_Effect_Explosion_C" (Transformation|GetActorTransform) false 0))

(fn ConstructionScript)

(fn ExplodeonHit
  (bind _returnvalue (Game|GetInstigator))
  (Networking|SwitchHasAuthority
    (:Authority
      (if (not (Variables|Default|GetIs%20Exploded))
        (Variables|Default|SetIs%20Exploded true) ; Don't allow explosion more than once!\nOtherwise 2 mines exploding next to each\nother get into an infinite loop.
        (Class|RadialForceComponent|FireImpulse (Variables|Default|GetRadialForce))
        ;[1 1 1] Set Instigator Controller if one exists
        (Utilities|IsValid _returnvalue
          (:Is%20Valid
            (LocalVariables|SetInstigator%20Controller (Game|GetInstigatorController _returnvalue)))
          (:Is%20Not%20Valid
            _))
        (Class|GameplayStatics|ApplyRadialDamagewithFalloff 25.0 0.0 (Transformation|GetActorLocation) 0.0 1e+03 1.0 0 0 self (LocalVariables|GetInstigator%20Controller) "ECC_Visibility")
        (Actor|DestroyActor)))))