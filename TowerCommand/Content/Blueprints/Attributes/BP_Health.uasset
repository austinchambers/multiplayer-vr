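; BP_Health is a health attribute component that tracks the health value of whatever owns it.
; DecreaseHealth subtracts a damage amount from HealthValue and clamps the result at zero.
; IsDestroyed reports whether health has reached zero, and IsAlive returns its inverse.
; The event graph holds only empty stubs, so health changes and state checks happen only when these functions are called.
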(event EventTick
  (params (DeltaSeconds :type Float%20%28single-precision%29)))

(event EventInitializeComponent)

(fn DecreaseHealth
  (params (Amount :type Float%20%28single-precision%29 :default 0.0))
  ;[1 1 1] Decrease health by damage amount.
  (Variables|Default|SetHealthValue (Math|Float|Max(Float) 0.0 (- (Variables|Default|GetHealthValue) Amount))))

(fn IsDestroyed
  ;[1 1 1] Return true if health has reached 0.
  (return (<= (Variables|Default|GetHealthValue) 0.0)))

(fn IsAlive
  (bind _is_destroyed (CallFunction|IsDestroyed))
  (return (not _is_destroyed)))