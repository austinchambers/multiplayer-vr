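; BP_Sub is a physics-driven player pawn, apparently a submarine, with health and VR headset support.
; Each tick it turns input into throttle, strafe, pitch and coupled roll-yaw forces, which the server applies unless destroyed; vertical and separate yaw inputs are disabled.
; Collision impulse over mass becomes damage that lowers health.
; Headset rotation drives the camera via a server call, and construction hands camera and scene capture to the parent class.
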(event Custom|Server%20Add%20Force%20and%20Torque
  (params (Force :type Vector :default "0, 0, 0") (Torque :type Vector :default "0, 0, 0"))
  ;[1 1 1] Per-frame processing.
  (Networking|SwitchHasAuthority
    (:Authority
      (bind _is_destroyed (CallFunction|IsDestroyed))
      (if _is_destroyed
        (Development|PrintString "dead")
        (else
          (Physics|AddForce Force "None")
          (Class|PrimitiveComponent|AddTorque Torque "None"))))))

(event Custom|Server%20Set%20HMD%20Rotation
  (params (Device%20Rotation :type Rotator :default "0, 0, 0"))
  (Variables|Default|SetHMDRotation Device%20Rotation))

(event EventBeginPlay)

(event EventTick
  (params (DeltaSeconds :type Float%20%28single-precision%29))
  ;[1 1 1] Set Camera Relative Rotation if HMD Enabled
  (if (Class|HeadMountedDisplayFunctionLibrary|IsHeadMountedDisplayEnabled)
    (CallFunction|ServerSetHMDRotation (.DeviceRotation (Class|HeadMountedDisplayFunctionLibrary|GetOrientationandPosition)))
    (Transformation|SetRelativeRotation (Variables|Default|GetHMDRotation) false))
  ;[1 1 1] Per-frame processing.
  (CallFunction|ApplyInputForces) ; Always apply input forces on the client side. Server will check if operation is legal.
)

(event EventHit
  (params (MyComp :type Primitive%20Component%20Object%20Reference) (Other :type Actor%20Object%20Reference) (OtherComp :type Primitive%20Component%20Object%20Reference) (bSelfMoved :type Boolean) (HitLocation :type Vector :default "0, 0, 0") (HitNormal :type Vector :default "0, 0, 0") (NormalImpulse :type Vector :default "0, 0, 0") (Hit :type Hit%20Result%20Structure%20%28by%20ref%29))
  ;[1 1 1] Trigger events on collisions.
  (Game|Damage|ApplyPointDamage self (* (/ (Math|Vector|VectorLength NormalImpulse) (Physics|GetMass)) (Variables|Default|GetCollision%20Damage%20Scale)) HitNormal Hit 0 Other))

(event EventAnyDamage
  (params (Damage :type Float%20%28single-precision%29) (DamageType :type Damage%20Type%20Object%20Reference) (InstigatedBy :type Controller%20Object%20Reference) (DamageCauser :type Actor%20Object%20Reference))
  ;[1 1 1] Deal with damage.
  (CallFunction|DecreaseHealth Damage))

(event Input|AxisEvents|InputAxisMoveRight
  (params (AxisValue :type Float%20%28single-precision%29))
  ;[1 1 1] Read player input to set throttle and torque
  (Variables|Default|SetRight%20Input AxisValue))

(event Input|AxisEvents|InputAxisMoveUp
  (params (AxisValue :type Float%20%28single-precision%29))
  ;[1 1 1] Read player input to set throttle and torque
)

(event Input|AxisEvents|InputAxisPitchRate
  (params (AxisValue :type Float%20%28single-precision%29))
  ;[1 1 1] Read player input to set throttle and torque
  (Variables|Default|SetPitch%20Input AxisValue))

(event Input|AxisEvents|InputAxisRollRate
  (params (AxisValue :type Float%20%28single-precision%29))
  ;[1 1 1] Read player input to set throttle and torque
  (Variables|Default|SetRoll%20Input AxisValue))

(event Input|AxisEvents|InputAxisYawRate
  (params (AxisValue :type Float%20%28single-precision%29))
  ;[1 1 1] Read player input to set throttle and torque
)

(event Input|AxisEvents|InputAxisMoveForward
  (params (AxisValue :type Float%20%28single-precision%29))
  ;[1 1 1] Read player input to set throttle and torque
  (Variables|Default|SetForward%20Input AxisValue))

(fn ConstructionScript
  ;[1 1 1] Set Scene Capture Variable for Parent Class (For outputting view to elsewhere)
  (Variables|Default|SetRiftSceneCapture (Variables|Default|GetSceneCaptureComponent2D))
  ;[1 1 1] Set Pawn's Camera for parent class
  (Variables|Default|SetRiftPawnCamera (Variables|Default|GetPawnCamera))
  (|CallParentFunction))

(fn ApplyInputForces
  (bind _returnvalue (Transformation|GetActorRightVector))
  (bind _returnvalue_2 (Transformation|GetActorForwardVector))
  (bind _returnvalue_3 (Transformation|GetActorUpVector))
  (bind _turn_input_torque (Variables|Default|GetTurn%20Input%20Torque))
  (bind _roll_input (Variables|Default|GetRoll%20Input))
  (bind _returnvalue_4 (* _roll_input _turn_input_torque))
  ;[1 1 1] Apply forces from player input
  (CallFunction|ServerAddForceandTorque (+ (+ (* _returnvalue_2 (* (Variables|Default|GetForward%20Input) (Variables|Default|GetForward%20Throttle%20Force))) (* _returnvalue_3 0.0)) (* _returnvalue (* (Variables|Default|GetRight%20Input) (Variables|Default|GetRight%20Throttle%20Force)))) (+ (+ (* (* _returnvalue_2 _returnvalue_4) -1.0) (* (* _returnvalue_3 _returnvalue_4) 0.6)) (* _returnvalue (* (Variables|Default|GetPitch%20Input) (Variables|Default|GetTurn%20Input%20Torque))))))