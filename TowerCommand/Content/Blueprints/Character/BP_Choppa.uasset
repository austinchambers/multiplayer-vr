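; BP_Choppa is a controllable character Blueprint, apparently a helicopter, with an attached scene capture camera.
; On BeginPlay it routes the SceneCapture2D output to a render target.
; Pressing G makes the first player controller unpossess its pawn, with no repossession here.
; A Rotate function, not called in these graphs, yaws the actor at a frame-rate-independent fixed rate for positive axis input only.
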(event EventBeginPlay
  (Variables|/Script/Engine.SceneCaptureComponent2D|SetTextureTarget (Variables|Default|GetSceneCapture2D1) (Variables|Default|GetRenderTarget)))

(event Input|ActionEvents|InputActionG
  (:Pressed
    (Pawn|UnPossess (Game|GetPlayerController 0))))

(fn ConstructionScript)

(fn Rotate
  (params (AxisValue :type Float%20%28single-precision%29))
  (bind _returnvalue (Transformation|GetActorRotation))
  (bind (_pitch _yaw _roll) (Class|KismetMathLibrary|BreakRot _returnvalue))
  (if (> AxisValue 0.0)
    (Transformation|SetActorRotation self (Class|KismetMathLibrary|MakeRot _pitch (+ (* 1.0 1e+02 (Utilities|Time|GetWorldDeltaSeconds)) _yaw) _roll))))