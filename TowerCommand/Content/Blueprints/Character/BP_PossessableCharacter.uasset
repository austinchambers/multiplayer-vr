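; Possessable character that carries a scene capture and can hand player control back to a stored return character.
; On BeginPlay it points the scene capture at its render target.
; The Possess input calls PossessToggle, which makes the stored player controller possess the return character, then clears both references.
; Only the return path is implemented, marked as temporary; PossessToggle does nothing when asked to possess.
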(event EventBeginPlay
  ;[1 1 1] Initialize Scene Capture
  (Variables|/Script/Engine.SceneCaptureComponent2D|SetTextureTarget (Variables|Default|GetSceneCapture) (Variables|Default|GetRenderTarget)))

(event Input|ActionEvents|InputActionPossess
  ;[1 1 1] Handle Possession (Temporarily only handles returns)
  (:Pressed
    (CallFunction|PossessToggle false)))

(fn ConstructionScript)

(fn PossessToggle
  (params (IsPossess :type Boolean))
  (if (not IsPossess)
    (Pawn|Possess (Variables|Default|GetPlayerControllerOwner) (Variables|Default|GetReturnCharacter))
    (Variables|Default|SetPlayerControllerOwner 0)
    (Variables|Default|SetReturnCharacter 0)))