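; BP_SubCharacter is a player-controlled submarine pawn moved by physics forces and torques.
; Input axes store forward, strafe, roll and pitch values, which ApplyInputForces turns into actor-relative force and torque every Tick.
; Roll input also drives a scaled yaw for banked turns, while vertical thrust and separate yaw input are disabled.
; Construction hands its SubSceneCaptureComponent2D to the parent class's SceneCapture variable.
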(event EventBeginPlay)

(event EventActorBeginOverlap
  (params (OtherActor :type Actor%20Object%20Reference)))

(event EventTick
  (params (DeltaSeconds :type Float%20%28single-precision%29))
  (CallFunction|ApplyInputForces))

(event Input|AxisEvents|InputAxisMoveRight
  (params (AxisValue :type Float%20%28single-precision%29))
  ;[1 1 1] Read player input to set throttle and torque
  (Variables|Default|SetRight%20Input AxisValue))

(event Input|AxisEvents|InputAxisMoveUp
  (params (AxisValue :type Float%20%28single-precision%29))
  ;[1 1 1] Read player input to set throttle and torque
)

(event Input|AxisEvents|InputAxisPitchRate
  (params (AxisValue :type Float%20%28single-precision%29))
  ;[1 1 1] Read player input to set throttle and torque
  (Variables|Default|SetPitch%20Input AxisValue))

(event Input|AxisEvents|InputAxisRollRate
  (params (AxisValue :type Float%20%28single-precision%29))
  ;[1 1 1] Read player input to set throttle and torque
  (Variables|Default|SetRoll%20Input AxisValue))

(event Input|AxisEvents|InputAxisYawRate
  (params (AxisValue :type Float%20%28single-precision%29))
  ;[1 1 1] Read player input to set throttle and torque
)

(event Input|AxisEvents|InputAxisMoveForward
  (params (AxisValue :type Float%20%28single-precision%29))
  ;[1 1 1] Read player input to set throttle and torque
  (Variables|Default|SetForward%20Input AxisValue))

(fn ConstructionScript
  ;[1 1 1] Set Scene Capture Variable for Parent Class
  (Variables|Default|SetSceneCapture (Variables|Default|GetSubSceneCaptureComponent2D))
  (|CallParentFunction))

(fn ApplyInputForces
  (bind _returnvalue (Transformation|GetActorRightVector))
  (bind _returnvalue_2 (Transformation|GetActorForwardVector))
  (bind _returnvalue_3 (Transformation|GetActorUpVector))
  (bind _turn_input_torque (Variables|Default|GetTurn%20Input%20Torque))
  (bind _roll_input (Variables|Default|GetRoll%20Input))
  (bind _returnvalue_4 (* _roll_input _turn_input_torque))
  ;[1 1 1] Apply forces from player input
  (Physics|AddForce (+ (+ (* _returnvalue_2 (* (Variables|Default|GetForward%20Input) (Variables|Default|GetForward%20Throttle%20Force))) (* _returnvalue_3 0.0)) (* _returnvalue (* (Variables|Default|GetRight%20Input) (Variables|Default|GetRight%20Throttle%20Force)))) "None")
  (Class|PrimitiveComponent|AddTorque (+ (+ (* (* _returnvalue_2 _returnvalue_4) -1.0) (* (* _returnvalue_3 _returnvalue_4) 0.6)) (* _returnvalue (* (Variables|Default|GetPitch%20Input) (Variables|Default|GetTurn%20Input%20Torque)))) "None"))