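; Player controller that detects which interactive object the controlled pawn is facing.
; Every tick it line-traces forward on the Camera channel, taking origin and direction from MyCharacter or, for any other pawn (the puppet), the actor transform.
; It caches the last BP_InteractiveObject hit and sends looking-at and not-looking-at calls only when the target changes or is lost.
; The trace debug-draws each frame.
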(event EventTick
  (params (DeltaSeconds :type Float%20%28single-precision%29))
  (CallFunction|LookatInteractiveObjects))

(fn ConstructionScript)

(fn LookatInteractiveObjects
  (bind _returnvalue (Pawn|GetControlledPawn))
  (bind _self self)
  (Utilities|IsValid _returnvalue
    (:Is%20Valid
      ;[1 1 1] If we're ray casting from MyCharacter
      (bind _asmy_character (Utilities|Casting|CastToMyCharacter _returnvalue)
        (:then
          (LocalVariables|SetWorldLocation (Transformation|GetWorldLocation _asmy_character))
          (LocalVariables|SetForwardVector (Math|Vector|GetForwardVector _asmy_character)))
        (:CastFailed
          ;[1 1 1] Ray Casting From Puppet
          (LocalVariables|SetWorldLocation (Transformation|GetActorLocation _returnvalue))
          (LocalVariables|SetForwardVector (Transformation|GetActorForwardVector _returnvalue))))
      ;[1 1 1] Cast a ray to see what you hit
      (bind (_outhit _returnvalue_2) (Collision|LineTraceByChannel (+ (* (LocalVariables|GetForwardVector) 75.0) (LocalVariables|GetWorldLocation)) (+ (* (LocalVariables|GetForwardVector) 2e+03) (LocalVariables|GetWorldLocation)) "TraceTypeQuery2" false 0 "ForOneFrame"))
      (if _returnvalue_2
        ;[1 1 1] Found InteractiveObject. If moving away from one IO to another, set "Not Looking" event in addition to "Looking At".
        (bind _asbp_interactive_object (Utilities|Casting|CastToBP_InteractiveObject (.HitActor (Collision|BreakHitResult _outhit)))
          (:then
            (if (!= _asbp_interactive_object (Variables|Default|GetLast%20Interactive%20Object))
              (Default|PlayerNotLookingat (Variables|Default|GetLast%20Interactive%20Object) _self)
              (Default|PlayerLookingat _asbp_interactive_object _self)
              (Variables|Default|SetLast%20Interactive%20Object _asbp_interactive_object)))
          (:CastFailed
            ;[1 1 1] Reset Last Interactive Object if Not Looking at One
            (Utilities|IsValid (Variables|Default|GetLast%20Interactive%20Object) :!label _label
              (:Is%20Valid
                (Default|PlayerNotLookingat (Variables|Default|GetLast%20Interactive%20Object) self)
                (Variables|Default|SetLast%20Interactive%20Object 0)))))
        (else
          (goto _label))))))