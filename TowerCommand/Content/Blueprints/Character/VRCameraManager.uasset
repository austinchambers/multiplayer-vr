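; VRCameraManager is a player camera manager that places the VR view relative to the player's BP_Sub pawn.
; Its BlueprintUpdateCamera override adds headset position to the CameraLocation relative location, transforms that offset into sub space and adds the sub's location.
; Camera rotation combines pawn rotation with headset rotation.
; Both headset position and rotation are scaled to a tenth, damping head movement.
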(event EventBeginPlay)

(event EventActorBeginOverlap
  (params (OtherActor :type Actor%20Object%20Reference)))

(event EventTick
  (params (DeltaSeconds :type Float%20%28single-precision%29)))

(fn ConstructionScript)

(fn BlueprintUpdateCamera
  (bind (_devicerotation _deviceposition) (Class|HeadMountedDisplayFunctionLibrary|GetOrientationandPosition))
  (bind _returnvalue (Game|Player|GetPlayerPawn 0))
  (bind _asbp_sub (Utilities|Casting|CastToBP_Sub _returnvalue))
  (return (+ (Math|Transform|TransformDirection (Transformation|GetActorTransform _asbp_sub) (+ (/ _deviceposition 1e+01) (Variables|/Script/Engine.SceneComponent|GetRelativeLocation (Variables|Default|GetCameraLocation)))) (Transformation|GetActorLocation _asbp_sub)) (Math|Rotator|CombineRotators (Transformation|GetActorRotation _returnvalue) (* _devicerotation 0.1)) true))