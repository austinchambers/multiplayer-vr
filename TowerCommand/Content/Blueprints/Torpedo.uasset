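; Torpedo projectile actor that travels in a straight line and explodes on timeout, hit or damage.
; The server launches it along local negative X via physics velocity and runs the fuse timer.
; An authority-only, once-guarded Explode applies radial falloff damage, then calls Exploded.
; Exploded spawns the explosion effect, destroys components and ends trails, delaying actor destruction so the trail lingers.
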(event Custom|Exploded
  ;[1 1 1] After torpedo explode event fires, spawn a particle effect for the explosion and
  ; destroy all parts of the torpedo except its trail.
  (Utilities|FlowControl|Sequence
    (:then_0
      (Game|SpawnActorfromClass "/Game/Blueprints/Blueprint_Effect_Explosion.Blueprint_Effect_Explosion_C" (Transformation|GetActorTransform) true 0))
    (:then_1
      (Components|DestroyComponent))
    (:then_2
      (Components|DestroyComponent))
    (:then_3
      (Components|DestroyComponent))
    (:then_4
      (Components|DestroyComponent))
    (:then_5
      (Effects|Particles|Trails|EndTrails))
    (:then_6
      (Utilities|FlowControl|Delay 1e+01)
      (Actor|DestroyActor))))

(event EventBeginPlay
  ;[1 1 1] The life of a torpedo. Nasty, brutish, and short.
  (Audio|Components|Audio|Play (Variables|Default|GetPulse) 0.0)
  (Networking|SwitchHasAuthority
    (:Authority
      (Physics|SetPhysicsLinearVelocity (Variables|Default|GetTorpedoBounds) (* (Math|Vector|Normalize (Math|Transform|TransformDirection (Transformation|GetActorTransform) "-1.000000, 0, 0")) (Variables|Default|GetTorpedo%20Speed)) false "None")
      (Utilities|FlowControl|Delay (Variables|Default|GetTORPEDO%20RUNTIME))
      (CallFunction|Explode false))))

(event EventHit
  (params (MyComp :type Primitive%20Component%20Object%20Reference) (Other :type Actor%20Object%20Reference) (OtherComp :type Primitive%20Component%20Object%20Reference) (bSelfMoved :type Boolean) (HitLocation :type Vector :default "0, 0, 0") (HitNormal :type Vector :default "0, 0, 0") (NormalImpulse :type Vector :default "0, 0, 0") (Hit :type Hit%20Result%20Structure%20%28by%20ref%29))
  ;[1 1 1] The life of a torpedo. Nasty, brutish, and short.
  (Networking|SwitchHasAuthority ; Only check collisions on server.
    (:Authority
      (CallFunction|Explode false))))

(event EventAnyDamage
  (params (Damage :type Float%20%28single-precision%29) (DamageType :type Damage%20Type%20Object%20Reference) (InstigatedBy :type Controller%20Object%20Reference) (DamageCauser :type Actor%20Object%20Reference))
  ;[1 1 1] The life of a torpedo. Nasty, brutish, and short.
  (Networking|SwitchHasAuthority ; Only check collisions on server.
    (:Authority
      (CallFunction|Explode false))))

(fn ConstructionScript)

(fn Explode
  (params (NewParam :type Boolean))
  (Networking|SwitchHasAuthority
    (:Authority
      (if (not (Variables|Default|GetIs%20Exploded))
        (Variables|Default|SetIs%20Exploded true)
        (Variables|Default|SetTorpedo%20Speed 0.0)
        (Class|GameplayStatics|ApplyRadialDamagewithFalloff 25.0 0.0 (Transformation|GetActorLocation) 0.0 1e+03 1.0 0 0 self (Game|GetInstigatorController (Variables|Actor|GetInstigator)) "ECC_Visibility")
        (CallFunction|Exploded)))))