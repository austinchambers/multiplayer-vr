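; VRGameMode is a game mode that assigns joining players to VR rift pawns already placed in the level.
; On PostLogin it gathers all BP_RiftPawn actors and picks one by an incrementing SpawnOrder index.
; It stores that pawn and index on the MyPlayerController as PermanentCharacter and PlayerIndex, then possesses the pawn.
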(event EventPostLogin
  (params (NewPlayer :type Player%20Controller%20Object%20Reference))
  (bind _spawn_order (Variables|Default|GetSpawn%20Order))
  ;[1 1 1] Spawn players at player starts
  (bind _outactors (Actor|GetAllActorsOfClass "/Game/Blueprints/Character/BP_RiftPawn.BP_RiftPawn_C")) ; Find the player starts in the level
  (bind _asbp_rift_pawn (Utilities|Casting|CastToBP_RiftPawn (Utilities|Array|Get(acopy) _outactors _spawn_order)))
  (bind _asmy_player_controller (Utilities|Casting|CastToMyPlayerController NewPlayer))
  (bind _output_get (Variables|/Game/Blueprints/Character/MyPlayerController.MyPlayerController_C|SetPermanentCharacter _asmy_player_controller _asbp_rift_pawn))
  (Variables|/Game/Blueprints/Character/MyPlayerController.MyPlayerController_C|SetPlayer%20Index _asmy_player_controller _spawn_order)
  (Pawn|Possess _asmy_player_controller _output_get)
  (Variables|Default|Setspawn%20order (+ (Variables|Default|Getspawn%20order) 1)))

(fn ConstructionScript)