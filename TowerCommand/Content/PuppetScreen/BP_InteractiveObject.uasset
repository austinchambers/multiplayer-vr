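; BP_InteractiveObject is an interactable object that highlights while a player looks at it, with an empty RespondToLook hook for custom reactions.
; Construction creates a dynamic material on DynamicHighlightMesh to drive its HighlightedAmount parameter.
; PlayerLookingAt stores the first looking controller as owner, turns on the highlight and calls the hook.
; PlayerNotLookingAt reverses this without checking which controller looked away; both print debug strings.
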(fn ConstructionScript
  (bind _returnvalue (Rendering|Material|CreateDynamicMaterialInstance (Variables|Default|GetDynamicHighlightMesh) 0 0 :!class /Script/Engine.PrimitiveComponent))
  (Variables|Default|SetDynamicHighlightMaterial _returnvalue))

(fn PlayerLookingat
  (params (Current%20Player%20Controller%20Looking :type My%20Player%20Controller%20Object%20Reference))
  ;[1 1 1] Handle LookAt State
  (Utilities|IsValid (Variables|Default|GetPlayerControllerOwner)
    (:Is%20Not%20Valid
      (Development|PrintString "Hello")
      (Variables|Default|SetPlayerControllerOwner Current%20Player%20Controller%20Looking)
      ;[1 1 1] Set Material Highlight
      (Rendering|Material|SetScalarParameterValue (Variables|Default|GetDynamicHighlightMaterial) "HighlightedAmount" 1.0 :!class /Script/Engine.MaterialInstanceDynamic)
      (CallFunction|RespondtoLook true Current%20Player%20Controller%20Looking))))

(fn PlayerNotLookingat
  (params (PlayerControllerNotLooking :type My%20Player%20Controller%20Object%20Reference))
  ;[1 1 1] Handle LookAt State
  (Utilities|IsValid (Variables|Default|GetPlayerControllerOwner)
    (:Is%20Valid
      (Development|PrintString "Goodbye")
      (Variables|Default|SetPlayerControllerOwner 0)
      ;[1 1 1] Update Material Instance
      (Rendering|Material|SetScalarParameterValue (Variables|Default|GetDynamicHighlightMaterial) "HighlightedAmount" 0.0 :!class /Script/Engine.MaterialInstanceDynamic)
      (CallFunction|RespondtoLook false))))

(fn RespondtoLook
  (params (IsLookingAt :type Boolean) (RelevantPlayerController :type My%20Player%20Controller%20Object%20Reference)))