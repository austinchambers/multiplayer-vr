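; BP_PuppetScreen is an in-world screen linked to a puppet helicopter that a player can rotate or possess.
; It supplies its bevel and screen mesh/material to parent-class highlight and render-target logic, and shows text prompts when looked at.
; Space toggles the Spin/Possess flag and label, while the F axis rotates the BP_Choppa regardless of mode.
; The Possess input hands the controlling player to the puppet and clears their look state.
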(event EventBeginPlay
  ;[1 1 1] Set the material / Render Target
  (Variables|Default|SetRenderScreenMesh (Variables|Default|GetPuppetScreenMesh))
  (Variables|Default|SetRenderScreenMaterial (Variables|Default|GetMaterialInst))
  (|CallParentFunction))

(event EventRespondtoLook
  (params (Relevant%20Player%20Index :type Integer) (IsLookingAt :type Boolean))
  ;[1 1 1] Event Override: Class-Specific Handling of Look Event
  (CallFunction|TextVisibility IsLookingAt))

(event Input|ActionEvents|InputActionSpace
  (:Pressed
    (CallFunction|ToggleMode)))

(event Input|ActionEvents|InputActionPossess
  (bind _controllingplayerindex (Variables|Default|GetControllingPlayerIndex))
  (bind _returnvalue (Game|GetPlayerController _controllingplayerindex))
  ;[1 1 1] Possess Associated Helicopter (For now, use 'G' key)
  (:Pressed
    (Utilities|IsValid _returnvalue
      (:Is%20Valid
        (Pawn|Possess _returnvalue (Variables|Default|GetPuppetToControl))
        (CallFunction|PlayerNotLookingat _controllingplayerindex)))))

(event Input|AxisEvents|InputAxisF
  (params (AxisValue :type Float%20%28single-precision%29))
  ;[1 1 1] Rotate Choppa
  (bind _asbp_choppa (Utilities|Casting|CastToBP_Choppa (Variables|Default|GetPuppetToControl)))
  (Default|Rotate _asbp_choppa AxisValue))

(fn ConstructionScript
  ;[1 1 1] Link Puppet Screen Bevel to Parent Class Highlight Object
  (Variables|Default|SetDynamicHighlightMesh (Variables|Default|GetPuppetScreen_Bevel))
  (|CallParentFunction))

(fn ToggleMode
  (bind _textrendermode (Variables|Default|GetTextRenderMode))
  (if (Variables|Default|GetSpinMode)
    (Rendering|Components|TextRender|SetText _textrendermode "Possess")
    (Variables|Default|SetSpinMode false)
    (else
      (Rendering|Components|TextRender|SetText _textrendermode "Spin")
      (Variables|Default|SetSpinMode true))))

(fn TextVisibility
  (params (IsVisible :type Boolean))
  (Rendering|SetVisibility (Variables|Default|GetTextRenderSpace) IsVisible false)
  (Rendering|SetVisibility (Variables|Default|GetTextRenderMode) IsVisible false))