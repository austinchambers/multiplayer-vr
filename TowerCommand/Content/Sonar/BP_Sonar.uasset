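; Sonar display actor that plots nearby targetable actors as dots on a screen mesh, relative to the current pawn.
; Construction derives the usable screen radius from mesh bounds and creates the sonar and player-dot materials.
; Tick, throttled by a half-second Delay as a stopgap, destroys and respawns the dots as static mesh components.
; Detection converts BPI_Targetable actors within range to normalized distance and yaw-relative angle, which SpawnDot turns into screen offsets.
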(event Custom|Detect%20and%20Draw%20Dots
  ;[1 1 1] Get info about other players and draw the dots
  (bind _detections (CallFunction|GetDetectionArray))
  (for _array_element _detections
    (CallFunction|SpawnDot (.x _array_element) (.y _array_element))))

(event EventActorBeginOverlap
  (params (OtherActor :type Actor%20Object%20Reference)))

(event EventTick
  (params (DeltaSeconds :type Float%20%28single-precision%29))
  ;[1 1 1] Destroy the dots and redraw after 0.5 sec
  (Utilities|FlowControl|Delay 0.5) ; Hacky for now, will sync to material instance later
  (CallFunction|DestroyDots)
  (CallFunction|DetectandDrawDots))

(fn ConstructionScript
  (bind (_min _max) (Components|StaticMesh|GetLocalBounds))
  (bind _screen_useable_ratio (Variables|ScreenProperties|GetScreen%20Useable%20Ratio))
  (bind _screen (Variables|Default|GetScreen))
  (bind _returnvalue (- _max _min))
  ;[1 1 1] Set the Screen's Transform
  (Variables|ScreenProperties|SetScreen%20Transform (Transformation|GetWorldTransform _screen))
  ;[1 1 1] Get Screen Dimensions
  (Variables|ScreenProperties|SetScreen%20Dimensions (Math|Vector2D|MakeVector2D (* _screen_useable_ratio (.x _returnvalue)) (* _screen_useable_ratio (.y _returnvalue))))
  ;[1 1 1] Set Screen Center
  (Variables|ScreenProperties|SetScreen%20Center (/ (Variables|ScreenProperties|GetScreen%20Dimensions) 2.0))
  ;[1 1 1] Get the screen's radius
  (Variables|ScreenProperties|SetScreen%20Radius (/ (Math|Float|Min(Float) (.x (Variables|ScreenProperties|GetScreen%20Dimensions)) (.y (Variables|ScreenProperties|GetScreen%20Dimensions))) 2.0))
  ;[1 1 1] Set the Sonar Material
  (Rendering|Material|CreateDynamicMaterialInstance _screen 0 (Variables|Rendering|GetSonar%20Material%20Instance) :!class /Script/Engine.PrimitiveComponent)
  ;[1 1 1] Set the self "dot" material
  (Rendering|Material|CreateDynamicMaterialInstance (Variables|Default|GetPlayer%20Dot) 0 (Variables|Rendering|GetSelf%20Material%20Instance) :!class /Script/Engine.PrimitiveComponent))

(fn GetAdjustedScreenInfo
  (params (Input%20Position :type Vector%202D%20Structure) (Input%20Width :type Float%20%28single-precision%29 :default 0.0) (Input%20Height :type Float%20%28single-precision%29 :default 0.0) (Ideal%20Screen%20Size :type Vector%202D%20Structure))
  (bind _screen_dimensions (Variables|ScreenProperties|GetScreen%20Dimensions))
  (bind _returnvalue (/ (.x _screen_dimensions) (.x Ideal%20Screen%20Size)))
  (bind _returnvalue_2 (/ (.y _screen_dimensions) (.y Ideal%20Screen%20Size)))
  (return (* Input%20Width _returnvalue) (* _returnvalue_2 Input%20Height) (Math|Vector2D|MakeVector2D (* (.x Input%20Position) _returnvalue) (* (.y Input%20Position) _returnvalue_2))))

(fn SpawnDot
  (params (Percent%20Distance :type Float%20%28single-precision%29 :default 0.0) (Angle%20 :type Float%20%28single-precision%29 :default 0.0))
  ;[1 1 1] Percent Distance * Radius gives us distance to point
  (LocalVariables|SetDistance%20To%20Point (* (Variables|ScreenProperties|GetScreen%20Radius) Percent%20Distance))
  ;[1 1 1] Spawn and Add to Array of References
  (bind _returnvalue (AddComponent|AddStaticMeshComponent false (Math|Conversions|ToTransform(Vector) (Math|Vector|MakeVector (* (Math|Trig|Sin(Degrees) Angle%20) (LocalVariables|GetDistance%20To%20Point)) (* (Math|Trig|Cos(Degrees) Angle%20) (LocalVariables|GetDistance%20To%20Point)) 0.0))))
  (Utilities|Array|Add (Variables|Default|GetDotReferences) _returnvalue)
  (return _returnvalue))

(fn GetDetectionArray
  (bind _detection_array (LocalVariables|GetDetection%20Array))
  ;[1 1 1] Scan for Targetable In Range
  (bind _outactors (Actor|GetAllActorswithInterface "/Game/Blueprints/Attributes/BPI_Targetable.BPI_Targetable_C"))
  (for _array_element _outactors
    (bind (_is_shown _detection_info) (CallFunction|GetDetectionInfoifRelevant _array_element))
    ;[1 1 1] Create Array
    (if _is_shown
      (Utilities|Array|Add _detection_array _detection_info)
      (return _detection_array))))

(fn GetDetectionInfoifRelevant
  (params (Detected%20Actor :type Actor%20Object%20Reference))
  (bind _returnvalue (Transformation|GetActorLocation Detected%20Actor))
  (bind _sonar_radius_distance (Variables|ScreenProperties|GetSonar%20Radius%20Distance))
  (bind _sonar_radius_distance_2 (Variables|ScreenProperties|GetSonar%20Radius%20Distance))
  (bind _current_pawn (Variables|Default|GetCurrent%20Pawn))
  (bind _current_pawn_2 (Variables|Default|GetCurrent%20Pawn))
  (bind _returnvalue_2 (Transformation|GetActorLocation _current_pawn_2))
  (bind _returnvalue_3 (- _returnvalue_2 _returnvalue))
  ;[1 1 1] Do nothing if current is self
  (if (not (== Detected%20Actor _current_pawn))
    ;[1 1 1] Get Distance
    (bind _output_get (LocalVariables|SetDetect%20Distance (Transformation|GetDistanceTo _current_pawn Detected%20Actor)))
    ;[1 1 1] If Distance is out, then do nothing
    (if (> _output_get _sonar_radius_distance)
      _
      (else
        ;[1 1 1] Otherwise, Get Scaled Distance
        (LocalVariables|SetScaled%20Distance (/ (LocalVariables|GetDetect%20Distance) _sonar_radius_distance))
        (LocalVariables|SetDetect%20Item%20Shown true)
        (LocalVariables|SetRelative%20Angle (* (Math|Float|%(Float) (+ (Class|KismetMathLibrary|DegAtan2 (/ (.y _returnvalue_3) _sonar_radius_distance_2) (/ (.x _returnvalue_3) _sonar_radius_distance_2)) 9e+01 (* (.yaw (Transformation|GetActorRotation (Variables|Default|GetCurrent%20Pawn))) -1.0)) 3.6e+02) -1.0))))
    (return (LocalVariables|GetDetect%20Item%20Shown) (Math|Vector2D|MakeVector2D (LocalVariables|GetScaled%20Distance) (LocalVariables|GetRelative%20Angle)))))

(fn DestroyDots
  (bind _dotreferences (Variables|Default|GetDotReferences))
  (for _array_element _dotreferences
    (Components|DestroyComponent _array_element))
  (Utilities|Array|Clear _dotreferences))