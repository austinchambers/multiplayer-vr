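; Debug HUD that draws a player-centered sonar in the top-left screen corner, with dots for nearby targetable actors.
; Each DrawHUD gathers BPI_Targetable actors, skips the player, and keeps those within the sonar radius.
; Their offsets are scaled into radar space and rotated by player pawn yaw so the radar turns with the player.
; Dots, player marker and radar are drawn as materials, scaled from a 1080p reference resolution.
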(event EventBeginPlay)

(event EventActorBeginOverlap
  (params (OtherActor :type Actor%20Object%20Reference)))

(event EventDrawHUD
  (params (SizeX :type Integer) (SizeY :type Integer))
  (Variables|Default|SetScreen%20Dimensions (Math|Vector2D|MakeVector2D (Math|Conversions|ToFloat(Integer) SizeX) (Math|Conversions|ToFloat(Integer) SizeY)))
  (CallFunction|DrawSonar "(X=300.000000,Y=300.000000)" "(X=0.000000,Y=0.000000)"))

(fn ConstructionScript
  ;[1 1 1] Set the Sonar Material
  (bind _returnvalue (Rendering|Material|CreateDynamicMaterialInstance (Variables|Default|GetScreen) 0 "/Game/Sonar/SonarDetectBase_Mat.SonarDetectBase_Mat" :!class /Script/Engine.PrimitiveComponent))
  (Variables|Default|SetSonarMaterialInstance _returnvalue))

(fn DrawSonarTexture
  (params (Position :type Vector%202D%20Structure) (Width :type Float%20%28single-precision%29 :default 0.0) (Height :type Float%20%28single-precision%29 :default 0.0) (ScreenSize :type Vector%202D%20Structure) (Material :type Material%20Instance%20Object%20Reference))
  (bind (_width _height _position) (CallFunction|GetAdjustedScreenInfo Position Width Height ScreenSize))
  (Class|HUD|DrawMaterialSimple Material (.x _position) (.y _position) _width _height 1.0 false))

(fn GetAdjustedScreenInfo
  (params (Input%20Position :type Vector%202D%20Structure) (Input%20Width :type Float%20%28single-precision%29 :default 0.0) (Input%20Height :type Float%20%28single-precision%29 :default 0.0) (Ideal%20Screen%20Size :type Vector%202D%20Structure))
  (bind _screen_dimensions (Variables|Default|GetScreen%20Dimensions))
  (bind _returnvalue (/ (.x _screen_dimensions) (.x Ideal%20Screen%20Size)))
  (bind _returnvalue_2 (/ (.y _screen_dimensions) (.y Ideal%20Screen%20Size)))
  (return (* Input%20Width _returnvalue) (* _returnvalue_2 Input%20Height) (Math|Vector2D|MakeVector2D (* (.x Input%20Position) _returnvalue) (* (.y Input%20Position) _returnvalue_2))))

(fn DrawSonar
  (params (Radar%20Size :type Vector%202D%20Structure) (Position :type Vector%202D%20Structure))
  (Variables|Default|SetSonar%20Start%20Location Position)
  ;[1 1 1] Scan for Targetable In Range
  (bind _outactors (Actor|GetAllActorswithInterface "/Game/Blueprints/Attributes/BPI_Targetable.BPI_Targetable_C"))
  (for _array_element _outactors
    (bind _actor (Utilities|IsDetectedActorinRange _array_element)
      (:In%20Range
        ;[1 1 1] Get Plot Location for Non Rotating Radars
        (bind (_radar_position _radar_center) (CallFunction|GetRadarPosition _actor (Math|Vector2D|MakeVector2D (.x Radar%20Size) (.y Radar%20Size))))
        (bind _radar_rotation (CallFunction|GetRadarRotation))
        ;[1 1 1] Rotate the Point around the center based on camera rotation
        (bind _new_point (CallFunction|RotatePoint _radar_position _radar_center _radar_rotation))
        ;[1 1 1] Take the start location of the radar and add the position offset
        (bind _new_offset (CallFunction|GetTempOffset _new_point))
        ;[1 1 1] Draw dot of detected object
        (CallFunction|DrawSonarTexture _new_offset 5.0 5.0 "(X=1920.000000,Y=1080.000000)" (Variables|Default|GetMonster%20Id)))))
  ;[1 1 1] Draw Main Player in the Center of Sonar
  (bind _new_offset_2 (CallFunction|GetTempOffset (Math|Vector2D|MakeVector2D (/ (.x Radar%20Size) 2.0) (/ (.y Radar%20Size) 2.0))))
  (CallFunction|DrawSonarTexture _new_offset_2 5.0 5.0 "(X=1920.000000,Y=1080.000000)" (Variables|Default|GetPlayer%20Id))
  ;[1 1 1] Draw Sonar over point
  (bind _new_offset_3 (CallFunction|GetTempOffset))
  (CallFunction|DrawSonarTexture _new_offset_3 (.x Radar%20Size) (.y Radar%20Size) "(X=1920.000000,Y=1080.000000)" (Variables|Default|GetRadar)))

(fn GetTempOffset
  (params (Offset :type Vector%202D%20Structure))
  (return (+ (Variables|Default|GetSonar%20Start%20Location) Offset)))

(fn GetRadarPosition
  (params (Detected%20Actor :type Actor%20Object%20Reference) (Radar%20Size :type Vector%202D%20Structure))
  (bind (_x _y) (Math|Vector2D|BreakVector2D Radar%20Size))
  (bind _returnvalue (Game|Player|GetPlayerPawn 0))
  (bind _returnvalue_2 (Transformation|GetActorLocation Detected%20Actor))
  (bind _sonarradiusdistance (Variables|Default|GetSonarRadiusDistance))
  (bind _returnvalue_3 (/ _y 2.0))
  (bind _returnvalue_4 (/ _x 2.0))
  (bind _returnvalue_5 (Transformation|GetActorLocation _returnvalue))
  (bind _returnvalue_6 (- _returnvalue_5 _returnvalue_2))
  (return (Math|Vector2D|MakeVector2D (+ (* _returnvalue_4 (/ (.x _returnvalue_6) _sonarradiusdistance)) _returnvalue_4) (+ _returnvalue_3 (* _returnvalue_3 (/ (.y _returnvalue_6) _sonarradiusdistance)))) (Math|Vector2D|MakeVector2D _returnvalue_4 _returnvalue_3)))

(fn GetRadarRotation
  (return (* (Math|Trig|DegreesToRadians (Math|Float|%(Float) (+ (.yaw (Transformation|GetActorRotation (Game|Player|GetPlayerPawn 0))) 9e+01) 3.6e+02)) -1.0)))

(fn RotatePoint
  (params (Point%20to%20Rotate :type Vector%202D%20Structure) (Center%20Point :type Vector%202D%20Structure) (Angle%20in%20Rad :type Float%20%28single-precision%29 :default 0.0))
  (return (Math|Vector2D|MakeVector2D (+ (.x Center%20Point) (- (* (Math|Trig|Cos(Radians) Angle%20in%20Rad) (- (.x Point%20to%20Rotate) (.x Center%20Point))) (* (Math|Trig|Sin(Radians) Angle%20in%20Rad) (- (.y Point%20to%20Rotate) (.y Center%20Point))))) (+ (.y Center%20Point) (+ (* (Math|Trig|Cos(Radians) Angle%20in%20Rad) (- (.y Point%20to%20Rotate) (.y Center%20Point))) (* (Math|Trig|Sin(Radians) Angle%20in%20Rad) (- (.x Point%20to%20Rotate) (.x Center%20Point))))))))